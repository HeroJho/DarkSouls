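; Player creature Blueprint whose own graph holds only debug key handlers for testing movement, time and damage.
; One key toggles global slow motion through a FlipFlop, and another triggers Jump.
; A third key caches the first BP_RamPage actor when TestObj is unset, then on later presses uses DKAttack to deal explosive knockback area damage with stun at that actor's location.
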(event EventBeginPlay)

(event Collision|EventActorBeginOverlap
  (params (OtherActor :type Actor%20Object%20Reference)))

(event EventTick
  (params (DeltaSeconds :type Float%20%28single-precision%29)))

(event Input|KeyboardEvents|DebugKey1
  (params (Key :type Key%20Structure :default "None") (ActionValue :type Input%20Action%20Value%20Structure))
  (:Pressed
    (if (== (Variables|Default|GetTestObj) 0)
      (bind _outactors (Actor|GetAllActorsOfClass "/Game/BluePrints/Creature/Monster/RamPage/BP_RamPage.BP_RamPage_C"))
      (Variables|Default|SetTestObj (Utilities|Array|Get(acopy) _outactors))
      (else
        (Class|DKAttackComponent|AOEDamage (Variables|Default|GetDK_Attack) (Transformation|GetActorLocation (Variables|Default|GetTestObj)) 1e+02 (Utilities|Struct|MakeS_DamageInfo 0 "Explosion" "KnockBack" false false false false 0 5.0) false)))))

(event Input|KeyboardEvents|DebugKeyJ
  (params (Key :type Key%20Structure :default "None") (ActionValue :type Input%20Action%20Value%20Structure))
  (:Pressed
    (Character|Jump)))

(event Input|KeyboardEvents|DebugKey0
  (params (Key :type Key%20Structure :default "None") (ActionValue :type Input%20Action%20Value%20Structure))
  (:Pressed
    (Utilities|FlowControl|FlipFlop
      (:A
        (Utilities|Time|SetGlobalTimeDilation 0.2))
      (:B
        (Utilities|Time|SetGlobalTimeDilation 1.0)))))

(fn ConstructionScript)